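; Burst-fire weapon Blueprint that overrides shooting to fire a series of shots per trigger press, followed by a delay.
; StartShooting fires the first shot, then a looping timer drives TakeBurstShot through a DoN counter until the burst count or ammo runs out.
; A delay timer then calls CanShoot to re-enable firing and reset the counter.
; StopShooting only prints a debug message, so releasing fire never interrupts a burst.
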(event `/Game/AllodsTestProject/Blueprints/I_WeaponInterface.StartShooting`
  ;[1 1 1] Переопределенная логика стрельбы
  (if (`self.IsCanTakeShoot`)
    (`self.TakeShot`)
    (set `self.IsCanShoot` false)
    (if (> (`self.BulletsCount`) 0)
      (bind _returnvalue (`KismetSystemLibrary.K2_SetTimerDelegate` (delegate `TakeBurstShot`) (`self.CalculateShootPeriod`) true))
      (set `self.ShootingTimerHandle` _returnvalue))))

(event `TakeBurstShot`
  (bind _returnvalue (- (`self.BurstShotsCount`) 1))
  ;[1 1 1] Переопределенная логика стрельбы
  (bind _counter (`/Engine/EditorBlueprintResources/StandardMacros.Do N` _returnvalue :!label _label)
    (:`Exit`
      (`self.TakeShot`)
      (if (not (and (!= _counter _returnvalue) (> (`self.BulletsCount`) 0)))
        (`KismetSystemLibrary.K2_ClearAndInvalidateTimerHandle` (`self.ShootingTimerHandle`))
        ;;[1 1 1] Задержка между очереями
        (bind _returnvalue_2 (`KismetSystemLibrary.K2_SetTimerDelegate` (delegate `CanShoot`) (`self.ShootingDelay`)))
        (set `self.ShootingTimerHandle` _returnvalue_2)))))

(event `CanShoot`
  ;[1 1 1] Переопределенная логика стрельбы
  (`KismetSystemLibrary.K2_ClearAndInvalidateTimerHandle` (`self.ShootingTimerHandle`))
  (set `self.IsCanShoot` true)
  (goto _label :!via `Reset`))

(event `/Game/AllodsTestProject/Blueprints/I_WeaponInterface.StopShooting`
  (`KismetSystemLibrary.PrintString` "Dont Interupt Burst" true true (struct :`R` 1.0 :`G` 0.953341 :`A` 1.0)))

(fn `UserConstructionScript`
  (`parent.UserConstructionScript`))