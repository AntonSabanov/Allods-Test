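; Single-shot weapon Blueprint that overrides the shooting logic to fire one shot per StartShooting call, with a cooldown between shots.
; StartShooting checks IsCanTakeShoot, calls TakeShot, clears IsCanShoot and starts a one-off timer lasting ShootingDelay.
; When the timer expires, the CanShooting event sets IsCanShoot back to true.
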(event `/Game/AllodsTestProject/Blueprints/I_WeaponInterface.StartShooting`
  ;[1 1 1] Переопределенная логика стрельбы
  (if (`self.IsCanTakeShoot`)
    (`self.TakeShot`)
    (set `self.IsCanShoot` false)
    (`KismetSystemLibrary.K2_SetTimerDelegate` (delegate `CanShooting`) (`self.ShootingDelay`))))

(event `CanShooting`
  ;[1 1 1] Переопределенная логика стрельбы
  (set `self.IsCanShoot` true))

(fn `UserConstructionScript`
  (`parent.UserConstructionScript`))