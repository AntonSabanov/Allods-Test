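; BP_AutoShootWeapon is a weapon Blueprint that overrides the parent's shooting logic to provide automatic fire.
; StartShooting fires a shot if allowed, then starts a looping timer at the period from CalculateShootPeriod and stores its handle.
; Each timer tick fires again through TakeAutoShoot, or calls StopShooting once a shot is no longer possible.
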(event `self.StartShooting`
  ;[1 1 1] Переопределенная логика стрельбы
  (if (`self.IsCanTakeShoot`)
    (`self.TakeShot`)
    (bind _returnvalue (`KismetSystemLibrary.K2_SetTimerDelegate` (delegate `TakeAutoShoot`) (`self.CalculateShootPeriod`) true))
    (set `self.ShootingTimerHandle` _returnvalue)))

(event `TakeAutoShoot`
  ;[1 1 1] Переопределенная логика стрельбы
  (if (`self.IsCanTakeShoot`)
    (`self.TakeShot`)
    (else
      (`self.StopShooting`))))

(fn `UserConstructionScript`
  (`parent.UserConstructionScript`))