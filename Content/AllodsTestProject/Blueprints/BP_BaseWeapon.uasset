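; Base weapon Blueprint that handles firing projectiles, ammo count and timed reloading.
; TakeShot triggers the shoot animation, spawns BP_BaseProjectile from the Sphere plus a camera-rotated offset, plays sound and decrements ammo.
; Reloading blocks shooting until a timer refills the magazine, and can be cancelled.
; StartShooting only logs, while StopShooting clears a shooting timer that is not set here; helpers expose readiness and RPM-based shot period.
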(event `/Game/AllodsTestProject/Blueprints/I_WeaponInterface.StartShooting`
  ;[1 1 1] Начало стрельбы (нажатие курка)
  (`KismetSystemLibrary.PrintString` "Start shooting" true true (struct :`R` 0.39038 :`G` 1.0 :`B` 0.422355 :`A` 1.0)))

(event `TakeShot`
  ;[1 1 1] Выстрел
  (`self.PlayShootAnimation`)
  (`self.SpawnProjectile`)
  (`/Engine/EditorBlueprintResources/StandardMacros.DecrementInt` (`self.BulletsCount`)
    (:`  `
      (`KismetSystemLibrary.PrintString` "Piu" true true (struct :`R` 1.0 :`G` 0.917572 :`A` 1.0)))))

(event `/Game/AllodsTestProject/Blueprints/I_WeaponInterface.StopShooting`
  ;[1 1 1] Конец стрельбы (отжатие курка)
  (`KismetSystemLibrary.PrintString` "Stop shooting" true true (struct :`R` 1.0 :`G` 0.013262 :`A` 1.0))
  (`KismetSystemLibrary.K2_ClearAndInvalidateTimerHandle` (`self.ShootingTimerHandle`))
  (set `self.ShootingTimerHandle` (struct)))

(event `/Game/AllodsTestProject/Blueprints/I_WeaponInterface.ReloadWeapon`
  ;[1 1 1] Перезарядка
  (if (`self.IsCanBeReloaded`)
    (`KismetSystemLibrary.PrintString` "Reloading" true true (struct :`R` 1.0 :`G` 0.85818 :`A` 1.0))
    (set `self.IsCanBeReloaded` false)
    (set `self.IsCanShoot` false)
    (bind _returnvalue (`KismetSystemLibrary.K2_SetTimerDelegate` (delegate `ReloadingComplete`) (`self.CooldownTime`)))
    (set `self.ReloadingTimerHandle` _returnvalue)))

(event `ReloadingComplete`
  ;[1 1 1] Перезарядка
  (set `self.BulletsCount` (`self.MaxBulletsCount`))
  (set `self.IsCanShoot` true)
  (set `self.IsCanBeReloaded` true))

(event `/Game/AllodsTestProject/Blueprints/I_WeaponInterface.CancelReloading`
  ;[1 1 1] Отмена перезарядки
  (`KismetSystemLibrary.K2_ClearAndInvalidateTimerHandle` (`self.ReloadingTimerHandle`))
  (set `self.ReloadingTimerHandle` (struct))
  (set `self.IsCanShoot` true)
  (set `self.IsCanBeReloaded` true))

(fn `CalculateShootPeriod`
  (returns (ReturnValue :type "Float (double-precision)"))
  (return (/ 60.0 (`self.RateOfFire`))))

(fn `IsCanReloading`
  (returns (CanReloading :type Boolean))
  (return (`self.IsCanBeReloaded`)))

(fn `IsCanShooting`
  (returns (CanShoot :type Boolean))
  (return (`self.IsCanShoot`)))

(fn `IsCanTakeShoot`
  (returns (CanTakeShoot :type Boolean))
  (return (and (`self.IsCanShoot`) (> (`self.BulletsCount`) 0))))

(fn `SpawnProjectile`
  (bind _returnvalue (`SceneComponent.K2_GetComponentRotation` (`self.PlayerCamera`)))
  (`|SpawnActorFromClass` "/Game/AllodsTestProject/Blueprints/BP_BaseProjectile.BP_BaseProjectile_C" (`KismetMathLibrary.MakeTransform` (+ (`SceneComponent.K2_GetComponentLocation` (`self.Sphere`)) (`KismetMathLibrary.GreaterGreater_VectorRotator` (`self.GunOffset`) _returnvalue)) _returnvalue) "AdjustIfPossibleButDontSpawnIfColliding" "OverrideRootScale" null null) ; Spawn projectile
  (`GameplayStatics.PlaySoundAtLocation` (`self.ShootSound`) (`self.K2_GetActorLocation`) (struct) 1.0 1.0 0.0 null null null) ; Play firing sound
)

(fn `UserConstructionScript`)